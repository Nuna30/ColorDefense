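; BP_APawnCreep is a creep pawn that uses AI navigation to walk to a hard-coded point when play begins, then heads for the world origin.
; MoveTo wraps AIMoveTo and, after a short delay on success or failure, calls itself with the origin, looping indefinitely with debug prints.
; An alternative MoveAround loop wanders between random reachable nearby points, but nothing that runs calls it.
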(event `self.ReceiveBeginPlay`
  (`self.MoveTo` (-1780.0 1780.0 5.0)))

(event `MoveTo`
  (params (Destination :type "Vector Structure"))
  (`|AIMoveTo` self Destination null
    (:`OnSuccess`
      (`KismetSystemLibrary.PrintString` "success")
      (`KismetSystemLibrary.Delay` 0.2))
    (:`OnFail`
      (`KismetSystemLibrary.PrintString` "fail")
      (`KismetSystemLibrary.Delay` 0.1)))
  (`self.MoveTo` (0.0 0.0 0.0)))

(event `MoveAround`
  (bind _output_get (set `self.Random Location` (`NavigationSystemV1.K2_GetRandomReachablePointInRadius` (`self.K2_GetActorLocation`) 1000.0 null null)))
  (`KismetSystemLibrary.PrintString` (`KismetStringLibrary.Conv_VectorToString` _output_get))
  (`|AIMoveTo` self _output_get null
    (:`OnSuccess`
      (`KismetSystemLibrary.PrintString` "Success")
      (`KismetSystemLibrary.Delay` 0.1))
    (:`OnFail`
      (`KismetSystemLibrary.PrintString` "Fail")
      (`KismetSystemLibrary.Delay` 0.1)))
  (`self.MoveAround`))

(fn `UserConstructionScript`)